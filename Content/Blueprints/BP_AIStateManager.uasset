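; BP_AIStateManager dispatches AI state changes to the hippo character that owns it.
; Its SetAIState event switches on the requested state (idle, roaming, eating, resting or running away), casts its owner to BP_Hippo and calls the matching OnState handler there.
; It keeps no state or behavior logic of its own, and does nothing if the owner is not a BP_Hippo.
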(event `SetAIState`
  (params (CurrentState :type "/Game/Blueprints/E_HippoState Enum" :default "NewEnumerator7"))
  (switch `/Game/Blueprints/E_HippoState` CurrentState
    (:`NewEnumerator7`
      (bind _asbp_hippo (cast `/Game/Blueprints/BP_Hippo` (`self.GetOwner`)))
      (`/Game/Blueprints/BP_Hippo.OnStateIdle()` _asbp_hippo))
    (:`NewEnumerator8`
      (bind _asbp_hippo_2 (cast `/Game/Blueprints/BP_Hippo` (`self.GetOwner`)))
      (`/Game/Blueprints/BP_Hippo.OnStateRoaming()` _asbp_hippo_2))
    (:`NewEnumerator2`
      (bind _asbp_hippo_3 (cast `/Game/Blueprints/BP_Hippo` (`self.GetOwner`)))
      (`/Game/Blueprints/BP_Hippo.OnStateEating()` _asbp_hippo_3))
    (:`NewEnumerator3`
      (bind _asbp_hippo_4 (cast `/Game/Blueprints/BP_Hippo` (`self.GetOwner`)))
      (`/Game/Blueprints/BPI_AnimalStateActions.OnStateResting()` _asbp_hippo_4))
    (:`NewEnumerator4`
      (bind _asbp_hippo_5 (cast `/Game/Blueprints/BP_Hippo` (`self.GetOwner`)))
      (`/Game/Blueprints/BP_Hippo.OnStateRunningAway()` _asbp_hippo_5))))

(fn `UserConstructionScript`)