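; BP_AlfaLion is an AI lion that, when flagged as alfa, patrols four locations in a loop with random pauses.
; AI perception detects BP_Hippo, stopping the lion for a one-time roar animation and sound.
; A separate Attack event, not called within this file, moves to the hippo and plays a bite.
; One-shot animations play directly on the mesh, then control returns to the Animation Blueprint; hit-reaction logic is left disconnected.
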(event `self.ReceiveBeginPlay`
  ;[0.8863 0.4549 0.7098 0.502] Begin play
  (if (`self.IsAlfa`)
    (`self.Patrolling`)))

(event `Patrolling`
  ;[0.8863 0.4549 0.7098 0.502] Patrolling
  (set `CharacterMovementComponent.MaxWalkSpeed` 600.0 (`self.CharacterMovement`))
  (`|AIMoveTo` self (`|GetArrayItem` (`self.PatrolLocatioons`) (`self.Locations`)) null 15.0 true
    (:`OnSuccess`
      (`KismetSystemLibrary.Delay` (`KismetMathLibrary.RandomFloatInRange` 1.0 5.0))
      (`self.Patrolling`)
      (`/Engine/EditorBlueprintResources/StandardMacros.IncrementInt` (`self.Locations`)
        (:`  `
          (if (== (`self.Locations`) 4)
            (set `self.Locations` 0)))))))

(event `self.AIPerception.OnTargetPerceptionUpdated`
  (params (Actor :type "Actor Object Reference") (Stimulus :type "AIStimulus Structure"))
  ;[0.8879 0.4564 0.7084 0.502] Sensing hippo
  (cast `/Game/Blueprints/BP_Hippo` Actor)
  (set `self.CanSeeHippo?` true)
  (if (`.bSuccessfullySensed` (break `AIStimulus` Stimulus))
    (bind _output_get (set `self.Should Attack?` true))
    (if _output_get
      (`/Engine/EditorBlueprintResources/StandardMacros.DoOnce` false :!label _label
        (:`Completed`
          (`MovementComponent.StopMovementImmediately` (`self.CharacterMovement`))
          (`self.Play Animation` false "/Game/AfricanAnimalsPack/LionAndLioness/Animations/ANIM_Lion_Roar.ANIM_Lion_Roar")
          (`GameplayStatics.PlaySoundAtLocation` "/Game/Audio/LionRoar/LionRoar_Cue.LionRoar_Cue" (`self.K2_GetActorLocation`) (struct) 1.0 1.0 0.0 null null null null)
          (`KismetSystemLibrary.Delay` 1.7)
          (`self.Stop Animation`)))
      (else
        (goto _label :!via `Reset`)))
    (else
      (set `self.CanSeeHippo?` false))))

(event `Attack`
  ;[0.8879 0.4564 0.7084 0.502] Sensing hippo
  (bind _asbp_hippo (cast `/Game/Blueprints/BP_Hippo` (stale `self.AIPerception.OnTargetPerceptionUpdated` Actor)))
  (if (`self.Should Attack?`)
    (set `self.Should Run?` true)
    (`|AIMoveTo` self (0.0 0.0 0.0) _asbp_hippo
      (:`OnSuccess`
        (`self.Play Animation` false "/Game/AfricanAnimalsPack/LionAndLioness/Animations/ANIM_Lion_Bite.ANIM_Lion_Bite")
        (`KismetSystemLibrary.Delay` 5.0)
        (`self.Stop Animation`)
        (if (`self.CanSeeHippo?`)
          _)))))

(fn `Play Animation`
  (params (bLooping :type Boolean) (NewAnimToPlay :type "AnimationAsset Object Reference"))
  (`SkeletalMeshComponent.PlayAnimation` (`self.Mesh`) NewAnimToPlay bLooping))

(fn `Stop Animation`
  (`SkeletalMeshComponent.SetAnimationMode` (`self.Mesh`) "AnimationBlueprint" true))

(fn `UserConstructionScript`)