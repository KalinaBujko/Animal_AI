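; Hippo animal AI that roams, grazes, rests, plays a swim animation in water, and flees from lions.
; DecideNextAction picks flee, rest, eat or roam by priority, fed by delay-looped energy, hunger and health counters.
; Grazing needs a matching surface underfoot, lion sightings or non-lethal hits trigger fleeing, and a forward trace on Tick redirects around obstacles.
; The attack branch and EvaluateFSM state machine are unfinished and unused.
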(event `self.ReceiveBeginPlay`
  ;[0.8863 0.4549 0.7098 0.502] BeginPlay
  (`self.Drain Energy`)
  (`self.Drain Hunger`)
  (`self.DecideNextAction` false))

(event `DecideNextAction`
  (params (`Skip Delay?` :type Boolean))
  ;[0.8879 0.4564 0.7084 0.502] Deciding next action
  (if (not `Skip Delay?`)
    (`KismetSystemLibrary.Delay` (`KismetMathLibrary.Conv_IntToDouble` (`KismetMathLibrary.RandomIntegerInRange` 1 5))))
  (if (`self.Should Run?`)
    (`self.Run Away`)
    (else
      ;;[0.8863 0.651 0.7922 0.502] Is tired?
      (if (`self.Is Tired?`)
        (`self.Rest`)
        (`self.Regain energy`)
        (else
          ;;[0.8863 0.651 0.7922 0.502] Is hungry?
          (if (`self.Is Hungry?`)
            (`self.EatFood`)
            (`self.Regain energy`)
            (`self.Add Health`)
            (else
              (`self.Roaming`)
              (`self.DecideNextAction` false))))))))

(event `Idle`
  ;[0.8863 0.4549 0.7098 0.502] State Machine
  ;;[0.8863 0.4549 0.7098 0.502] Idle
  (`MovementComponent.StopMovementImmediately` (`self.CharacterMovement`) :!label _label)
  (`KismetSystemLibrary.Delay` 5.0)
  (`self.DecideNextAction` false))

(event `ExecuteCurrentState`
  ;[0.8863 0.4549 0.7098 0.502] State Machine
  (switch `/Game/Blueprints/E_HippoState` (`self.CurrentState`)))

(event `/Game/Blueprints/BPI_AnimalStateActions.OnStateIdle()`
  ;[0.8863 0.4549 0.7098 0.502] State Machine
  ;;[0.8863 0.4549 0.7098 0.502] Idle
  (goto _label))

(event `/Game/Blueprints/BPI_AnimalStateActions.OnStateRoaming()`
  ;[0.8863 0.4549 0.7098 0.502] State Machine
  ;;[0.8863 0.4549 0.7098 0.502] Roaming
  (set `CharacterMovementComponent.MaxWalkSpeed` 130.0 (`self.CharacterMovement`) :!label _label_2)
  (`|AIMoveTo` self (`NavigationSystemV1.K2_GetRandomReachablePointInRadius` (`self.K2_GetActorLocation`) 1500.0 null null) null
    (:`then`
      (`KismetSystemLibrary.Delay` (`KismetMathLibrary.RandomFloatInRange` 1.0 15.0))
      (`self.DecideNextAction` false))))

(event `Roaming`
  ;[0.8863 0.4549 0.7098 0.502] State Machine
  ;;[0.8863 0.4549 0.7098 0.502] Roaming
  (goto _label_2))

(event `/Game/Blueprints/BPI_AnimalStateActions.OnStateEating()`
  ;[0.8863 0.4549 0.7098 0.502] State Machine
  ;;[0.8863 0.4549 0.7098 0.502] Eating
  (bind _can_eat_ (`self.Can Eat` :!label _label_3)
    (:`Out`
      (if _can_eat_
        (`MovementComponent.StopMovementImmediately` (`self.CharacterMovement`))
        (`self.Add Hunger`)
        (`self.Play Animation` "/Game/AfricanAnimalsPack/Hippopotamus/Animations/ANIM_Hippopotamus_GrazeDown.ANIM_Hippopotamus_GrazeDown")
        (`KismetSystemLibrary.Delay` 0.6)
        (`self.Play Animation` "/Game/AfricanAnimalsPack/Hippopotamus/Animations/ANIM_Hippopotamus_Graze.ANIM_Hippopotamus_Graze")
        (`KismetSystemLibrary.Delay` 0.6)
        (`self.Play Animation` "/Game/AfricanAnimalsPack/Hippopotamus/Animations/ANIM_Hippopotamus_IdleChew.ANIM_Hippopotamus_IdleChew" true)
        (`KismetSystemLibrary.Delay` (`KismetMathLibrary.Conv_IntToDouble` (`KismetMathLibrary.RandomIntegerInRange` 3 10)))
        (`self.Stop Animation`)
        (set `self.Is Hungry?` false)
        (`self.Drain Hunger`)
        (`self.DecideNextAction` false)
        (else
          (`self.DecideNextAction` false)
          (set `self.Is Hungry?` false)
          (`KismetSystemLibrary.Delay` 5.0)
          (set `self.Is Hungry?` true))))))

(event `EatFood`
  ;[0.8863 0.4549 0.7098 0.502] State Machine
  ;;[0.8863 0.4549 0.7098 0.502] Eating
  (goto _label_3))

(event `/Game/Blueprints/BPI_AnimalStateActions.OnStateResting()`
  ;[0.8863 0.4549 0.7098 0.502] State Machine
  ;;[0.8863 0.4549 0.7098 0.502] Resting
  (`MovementComponent.StopMovementImmediately` (`self.CharacterMovement`) :!label _label_4)
  (`self.Play Animation` "/Game/AfricanAnimalsPack/Hippopotamus/Animations/ANIM_Hippopotamus_GoToRest.ANIM_Hippopotamus_GoToRest")
  (`KismetSystemLibrary.Delay` 1.2)
  (`self.Play Animation` "/Game/AfricanAnimalsPack/Hippopotamus/Animations/ANIM_Hippopotamus_Resting.ANIM_Hippopotamus_Resting" true)
  (`KismetSystemLibrary.Delay` (`KismetMathLibrary.Conv_IntToDouble` (`KismetMathLibrary.RandomIntegerInRange` 50 120)))
  (`self.Play Animation` "/Game/AfricanAnimalsPack/Hippopotamus/Animations/ANIM_Hippopotamus_RestingToGoBackUp.ANIM_Hippopotamus_RestingToGoBackUp")
  (`KismetSystemLibrary.Delay` 1.7)
  (`self.Stop Animation`)
  (set `self.Is Tired?` false)
  (`self.DecideNextAction` false)
  (`self.Drain Energy`))

(event `Rest`
  ;[0.8863 0.4549 0.7098 0.502] State Machine
  ;;[0.8863 0.4549 0.7098 0.502] Resting
  (goto _label_4))

(event `/Game/Blueprints/BPI_AnimalStateActions.OnStateRunningAway()`
  ;[0.8863 0.4549 0.7098 0.502] State Machine
  ;;[0.8863 0.4549 0.7098 0.502] Running Away
  (set `CharacterMovementComponent.MaxWalkSpeed` 800.0 (`self.CharacterMovement`) :!label _label_5)
  (`|AIMoveTo` self (`NavigationSystemV1.K2_GetRandomReachablePointInRadius` (`self.K2_GetActorLocation`) (`KismetMathLibrary.RandomFloatInRange` 10000.0 20000.0) null null) null
    (:`then`
      (set `self.Should Run?` false)
      (`self.DecideNextAction` false))))

(event `Run Away`
  ;[0.8863 0.4549 0.7098 0.502] State Machine
  ;;[0.8863 0.4549 0.7098 0.502] Running Away
  (goto _label_5))

(event `Drain Energy`
  ;[0.8879 0.4564 0.7084 0.502] Draining energy -125s
  (if (not (`self.Is Tired?`))
    (bind _output_get (set `self.Energy` (`KismetMathLibrary.Clamp` (- (`self.Energy`) (`self.Energy Drain`)) 0 (`self.Max Energy`))))
    (if (== _output_get 0)
      (set `self.Is Tired?` true)
      (`self.DecideNextAction` false)
      (else
        (`KismetSystemLibrary.Delay` 1.0)
        (`self.Drain Energy`)))))

(event `Regain energy`
  ;[0.8879 0.4564 0.7084 0.502] Regain energy - 50s
  (if (`self.Is Tired?`)
    (bind _output_get (set `self.Energy` (`KismetMathLibrary.Clamp` (+ (`self.Energy`) (`self.Energy Gain`)) 0 (`self.Max Energy`))))
    (if (not (== _output_get (`self.Max Energy`)))
      (`KismetSystemLibrary.Delay` 1.0)
      (`self.Regain energy`))))

(event `Drain Hunger`
  ;[0.8879 0.4564 0.7084 0.502] Drain hunger
  (if (not (`self.Is Hungry?`))
    (bind _output_get (set `self.Hunger` (`KismetMathLibrary.Clamp` (- (`self.Hunger`) (`self.Hunger Drain`)) 0 (`self.Max Hunger`))))
    (if (== _output_get 0)
      (set `self.Is Hungry?` true)
      (`self.DecideNextAction` false)
      (else
        (`KismetSystemLibrary.Delay` 1.0)
        (`self.Drain Hunger`)))))

(event `Add Hunger`
  ;[0.8879 0.4564 0.7084 0.502] Regain hunger
  (if (`self.Is Hungry?`)
    (bind _output_get (set `self.Hunger` (`KismetMathLibrary.Clamp` (+ (`self.Hunger`) (`self.Hunger Gain`)) 0 (`self.Max Hunger`))))
    (if (not (== _output_get (`self.Max Hunger`)))
      (`KismetSystemLibrary.Delay` 1.0)
      (`self.Add Hunger`))))

(event `self.CapsuleComponent.OnComponentBeginOverlap`
  (params (OverlappedComponent :type "PrimitiveComponent Object Reference") (OtherActor :type "Actor Object Reference") (OtherComp :type "PrimitiveComponent Object Reference") (OtherBodyIndex :type Integer) (bFromSweep :type Boolean) (SweepResult :type "HitResult Structure (by ref)"))
  ;[0.8879 0.4564 0.7084 0.502] Swimming
  (cast `/Game/Blueprints/BP_Water` OtherActor)
  (`self.Play Animation` "/Game/AfricanAnimalsPack/Hippopotamus/Animations/ANIM_Hippopotamus_Swim.ANIM_Hippopotamus_Swim" true))

(event `self.CapsuleComponent.OnComponentEndOverlap`
  (params (OverlappedComponent :type "PrimitiveComponent Object Reference") (OtherActor :type "Actor Object Reference") (OtherComp :type "PrimitiveComponent Object Reference") (OtherBodyIndex :type Integer))
  ;[0.8879 0.4564 0.7084 0.502] Swimming
  (cast `/Game/Blueprints/BP_Water` OtherActor)
  (`self.Stop Animation`))

(event `Taking Damage`
  (bind _charactermovement (`self.CharacterMovement`))
  ;[0.8879 0.4564 0.7084 0.502] Taking damage
  (if (not (`self.Is Dead?`))
    (bind _output_get (set `self.Health` (`KismetMathLibrary.Clamp` (- (`self.Health`) (`self.Damage`)) 0 (`self.Max Health`))))
    (`GameplayStatics.PlaySoundAtLocation` "/Game/Audio/TakingDamage/TakeDamage_Cue.TakeDamage_Cue" (`self.K2_GetActorLocation`) (struct) 1.0 1.0 0.0 null null null null)
    (if (== _output_get 0)
      (`MovementComponent.StopMovementImmediately` _charactermovement)
      (set `self.Is Dead?` true)
      (`self.Play Animation` "/Game/AfricanAnimalsPack/Hippopotamus/Animations/ANIM_Hippopotamus_Death.ANIM_Hippopotamus_Death")
      (`KismetSystemLibrary.Delay` 2.3)
      (`CharacterMovementComponent.DisableMovement` (`self.CharacterMovement`))
      (`KismetSystemLibrary.Delay` (`KismetMathLibrary.Conv_IntToDouble` (`KismetMathLibrary.RandomIntegerInRange` 60 120)))
      (`self.K2_DestroyActor`)
      (else
        (`MovementComponent.StopMovementImmediately` _charactermovement)
        (`self.Play Animation` "/Game/AfricanAnimalsPack/Hippopotamus/Animations/ANIM_Hippopotamus_GetHit.ANIM_Hippopotamus_GetHit")
        (set `self.Should Run?` true)
        (`KismetSystemLibrary.Delay` 1.0)
        (`self.Stop Animation`)
        (if (not (`self.Is Dead?`))
          (`self.DecideNextAction` false))))))

(event `Add Health`
  ;[0.8879 0.4564 0.7084 0.502] Regen health
  (if (and (< (`self.Health`) (`self.Max Health`)) (not (`self.Should Run?`)))
    (bind _output_get (set `self.Health` (`KismetMathLibrary.Clamp` (+ (`self.Health`) (`self.Health Gain`)) 0 (`self.Max Health`))))
    (if (not (== _output_get (`self.Max Health`)))
      (`KismetSystemLibrary.Delay` 1.0 :!label _label_6)
      (`self.Add Health`))
    (else
      (goto _label_6))))

(event `self.PawnSensing.OnSeePawn`
  (params (Pawn :type "Pawn Object Reference"))
  ;[0.8879 0.4564 0.7084 0.502] Detect predator
  (cast `/Game/Blueprints/BP_Lion` Pawn)
  (bind _output_get (set `self.Should Run?` true))
  (if _output_get
    (`KismetSystemLibrary.PrintString` "biegne")
    (`self.Run Away`)
    (else
      (`self.DecideNextAction` false))))

(event `self.ReceiveHit`
  (params (MyComp :type "PrimitiveComponent Object Reference") (Other :type "Actor Object Reference") (OtherComp :type "PrimitiveComponent Object Reference") (bSelfMoved :type Boolean) (HitLocation :type "Vector Structure") (HitNormal :type "Vector Structure") (NormalImpulse :type "Vector Structure") (Hit :type "HitResult Structure (by ref)"))
  ;[0.8879 0.4564 0.7084 0.502] Being hit
  (cast `/Game/Blueprints/BP_Lion` Other)
  (set `self.Damage` 10)
  (`self.Taking Damage`))

(event `self.ReceiveTick`
  (params (DeltaSeconds :type "Float (single-precision)"))
  ;[0.8863 0.4549 0.7098 0.502] Avoiding obstacles
  (bind (_outhit _returnvalue) (`KismetSystemLibrary.LineTraceSingle` :`Start` (`self.K2_GetActorLocation`) :`End` (+ (`self.K2_GetActorLocation`) (* (`self.GetActorForwardVector`) (`KismetMathLibrary.RandomFloatInRange` 300.0 400.0))) :`TraceChannel` "TraceTypeQuery1" :`bIgnoreSelf` false))
  (`/Engine/EditorBlueprintResources/StandardMacros.IsValid` (`.HitActor` (`GameplayStatics.BreakHitResult` _outhit))
    (:`Is Valid`
      (if _returnvalue
        (`|AIMoveTo` self (`NavigationSystemV1.K2_GetRandomReachablePointInRadius` (`self.K2_GetActorLocation`) 300.0 null null) null
          (:`then`
            (`KismetSystemLibrary.Delay` (`KismetMathLibrary.RandomFloatInRange` 1.0 5.0))
            (`self.DecideNextAction` false)))))))

(fn `EvaluateFSM`
  (if (`self.IsBusy`)
    (return)
    (else
      ;[0.8879 0.6514 0.7913 0.502] Should run?
      (if (not (`self.Should Run?`))
        ;[0.8879 0.6514 0.7913 0.502] Is hungry?
        (if (not (`self.Is Hungry?`))
          ;[0.8879 0.6514 0.7913 0.502] Is tired?
          (if (`self.Is Tired?`)
            _))))))

(fn `Play Animation`
  (params (Animation :type "AnimationAsset Object Reference") (`Should loop?` :type Boolean))
  (`SkeletalMeshComponent.PlayAnimation` (`self.Mesh`) Animation `Should loop?`))

(fn `Stop Animation`
  (`SkeletalMeshComponent.SetAnimationMode` (`self.Mesh`) "AnimationBlueprint" true))

(fn `UserConstructionScript`)